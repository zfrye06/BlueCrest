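; Game instance for Sneaky Snek that handles menu flow, player preferences and multiplayer sessions.
; Events create and show the main, join, host and options menus plus a loading screen.
; A "userpref" save slot is loaded into PlayerStatus, or created if missing.
; Session events host, join and destroy games; hosting opens Lobby as a listen server from the async node's immediate output, without waiting for success.
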(event Custom|ShowMainMenu
  (bind _returnvalue (Game|GetPlayerController 0))
  ;[1 1 1] Show main menu and set input mode to UI only
  (bind _returnvalue_2 (UserInterface|CreateWidget "/Game/UI/MainMenu.MainMenu_C" _returnvalue))
  (bind _output_get (Variables|Menus|SetMainMenuRef _returnvalue_2))
  (UserInterface|Viewport|AddtoViewport _output_get 0)
  (Input|SetInputModeUIOnly _returnvalue _output_get false)
  (Variables|/Script/Engine.PlayerController|SetbShowMouseCursor _returnvalue true))

(event Custom|ShowJoinMenu
  ;[1 1 1] Shows join menu, hides main menu
  (bind _returnvalue (UserInterface|CreateWidget "/Game/UI/JoinGameMenu.JoinGameMenu_C" (Game|GetPlayerController 0)))
  (Widget|RemovefromParent (Variables|Menus|GetMainMenuRef))
  (UserInterface|Viewport|AddtoViewport _returnvalue 0))

(event Custom|ShowHostMenu
  ;[1 1 1] Show Host Menu
  (bind _returnvalue (UserInterface|CreateWidget "/Game/UI/HostMenu.HostMenu_C" (Game|GetPlayerController 0)))
  (Widget|RemovefromParent (Variables|Menus|GetMainMenuRef))
  (UserInterface|Viewport|AddtoViewport _returnvalue 0))

(event Custom|HostGame
  (params (PlayerLimit :type Integer) (isLan? :type Boolean))
  ;[1 1 1] Attempts to host a game
  (|Session (Game|GetPlayerController 0) PlayerLimit isLan?
    (:then
      (Game|OpenLevel(byName) "Lobby" true "listen")
      (Development|PrintString "SessionCreated" :!label _label))
    (:OnSuccess
      (goto _label))
    (:OnFailure
      (Development|PrintString "Session Create Failed"))))

(event Custom|JoinSession
  (params (Session :type Blueprint%20Session%20Result%20Structure))
  ;[1 1 1] Joins a session
  (|JoinSession (Game|GetPlayerController 0) Session
    (:then
      (CallFunction|ShowLoadingScreen))
    (:OnSuccess
      (Development|PrintString "Joined Session"))
    (:OnFailure
      (Development|PrintString "Session Join Failure"))))

(event Custom|ShowLoadingScreen
  ;[1 1 1] Shows the loading screen
  (bind _returnvalue (UserInterface|CreateWidget "/Game/UI/LoadingScreen.LoadingScreen_C" (Game|GetPlayerController 0)))
  (bind _output_get (Variables|Menus|SetLoadingScreenRef _returnvalue))
  (UserInterface|Viewport|AddtoViewport _output_get 0))

(event Custom|ShowOptionsMenu
  ;[1 1 1] Adds the options menu to the viewport
  (Viewport|RemoveAllWidgets)
  (bind _returnvalue (UserInterface|CreateWidget "/Game/UI/Options.Options_C"))
  (UserInterface|Viewport|AddtoViewport _returnvalue 0))

(event Custom|OpenSession
  (params (Players :type Integer) (Lan? :type Boolean))
  ;[1 1 1] Opens the session
  (|Session (Game|GetPlayerController 0) Players Lan?
    (:OnSuccess
      (Development|PrintString "Session Created!"))))

(event Custom|CheckSaveGame
  ;[1 1 1] Checks for a preferences save, if one does not exist, it creates one.
  (bind _returnvalue (SaveGame|DoesSaveGameExist "userpref"))
  (if _returnvalue
    (bind _returnvalue_2 (SaveGame|LoadGamefromSlot "userpref"))
    (bind _assnek_preferences (Utilities|Casting|CastToSnekPreferences _returnvalue_2))
    (Variables|Default|SetPreferences _assnek_preferences)
    (Utilities|Struct|SetmembersinPlayerStatus (Variables|Default|GetPlayerStatus) (Variables|/Game/Blueprints/Game/SnekPreferences.SnekPreferences_C|GetPreferedFaction (Variables|Default|GetPreferences)) false (Variables|/Game/Blueprints/Game/SnekPreferences.SnekPreferences_C|GetDefaultNickname (Variables|Default|GetPreferences)))
    (else
      (bind _returnvalue_3 (SaveGame|CreateSaveGameObject "/Game/Blueprints/Game/SnekPreferences.SnekPreferences_C"))
      (bind _assnek_preferences_2 (Utilities|Casting|CastToSnekPreferences _returnvalue_3))
      (bind _output_get (Variables|Default|SetPreferences _assnek_preferences_2))
      (SaveGame|SaveGametoSlot _output_get "userpref"))))

(event Custom|DestroySession
  (params (NewParam :type Player%20Controller%20Object%20Reference))
  ;[1 1 1] Destroys the play session
  (|DestroySession NewParam
    (:then
      (Game|OpenLevel(byName) "MainMenuMap"))))