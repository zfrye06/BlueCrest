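; Game mode for Sneaky Snek that starts the match once the configured player count connects and splits players into killers and town.
; Tracks controllers through login, swap from lobby and logout, carrying lobby status into the game controller.
; Role assignment boosts killer odds for players preferring that faction, deals each a unique random class and gives killers a knife.
; That class then determines each player's pawn, tagged PlayerStart and UI setup.
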(event Custom|LoadPlayers
  (bind ___chance (Utilities|%ChancetobeKiller))
  (bind _availableclasses (Variables|Default|GetAvailableClasses))
  (bind _returnvalue (Utilities|Array|Length _availableclasses))
  (bind _returnvalue_2 (- _returnvalue 1))
  (bind _returnvalue_3 (Math|Random|RandomInteger _returnvalue_2))
  (bind _item (Utilities|Array|Get(acopy) _availableclasses _returnvalue_3))
  ;[1 1 1] Assigns the player to a team and sets their class
  (if (not (< (Utilities|Array|Length (Variables|Default|GetConnectedControllers)) 1))
    (for _array_element (Variables|Default|GetConnectedControllers)
      (bind _assneaky_player_controller (Utilities|Casting|CastToSneakyPlayerController _array_element))
      (switch Utilities|FlowControl|Switch|SwitchonFactions (.FactionPreference (Utilities|Struct|BreakPlayerStatus (Variables|/Game/Blueprints/Game/SneakyPlayerController.SneakyPlayerController_C|GetPlayerStatus _assneaky_player_controller)))
        (:NewEnumerator0
          (Variables|Default|SetChanceToBeKiller ___chance))
        (:NewEnumerator1
          (Variables|Default|SetChanceToBeKiller (* ___chance 1.25))))
      (if (< (Math|Random|RandomFloat) (Variables|Default|GetChanceToBeKiller))
        (bind _structout (Utilities|Struct|SetmembersinDudeClass _item true))
        (Variables|Default|SetCurrentClass _structout)
        (Math|Integer|IncrementInt (Variables|RoleCounts|GetKillers)
          (:%20%20
            _))
        (else
          (bind _output_get (Variables|Default|SetCurrentClass _item))
          (Math|Integer|IncrementInt (Variables|RoleCounts|GetTown)
            (:%20%20
              _))))
      (Utilities|Array|RemoveItem (Variables|Default|GetAvailableClasses) _output_get)
      (Default|SetClass _assneaky_player_controller (Variables|Default|GetCurrentClass))
      (Default|SetClassServer _assneaky_player_controller (Variables|Default|GetCurrentClass)))
    (Development|PrintString "Assigned Player Roles")))

(event EventPostLogin
  (params (NewPlayer :type Player%20Controller%20Object%20Reference))
  (Utilities|Array|Add (Variables|Default|GetConnectedControllers) NewPlayer)
  (Development|PrintString "Added player"))

(event EventOnSwapPlayerControllers
  (params (OldPC :type Player%20Controller%20Object%20Reference) (NewPC :type Player%20Controller%20Object%20Reference))
  ;[1 1 1] Listens for player controller swap
  (bind _aslobby_player_controller (Utilities|Casting|CastToLobbyPlayerController OldPC)
    (:then
      (bind _assneaky_player_controller (Utilities|Casting|CastToSneakyPlayerController NewPC)
        (:then
          (Variables|/Game/Blueprints/Game/SneakyPlayerController.SneakyPlayerController_C|SetPlayerStatus _assneaky_player_controller (Variables|/Game/Blueprints/Lobby/LobbyPlayerController.LobbyPlayerController_C|GetStatus _aslobby_player_controller))
          (Utilities|Array|Add (Variables|Default|GetConnectedControllers) NewPC))
        (:CastFailed
          (Utilities|Array|Add (Variables|Default|GetConnectedControllers) NewPC :!label _label))))
    (:CastFailed
      (goto _label))))

(event EventBeginPlay
  ;[1 1 1] Game Settings
  (bind _assneaky_snek_game_instance (Utilities|Casting|CastToSneakySnekGameInstance (Game|GetGameInstance)))
  (Variables|Default|SetGameSettings (Variables|/Game/Blueprints/Game/SneakySnekGameInstance.SneakySnekGameInstance_C|GetGameSettings _assneaky_snek_game_instance)))

(event EventOnSetMatchState
  (params (NewState :type Name))
  ;[1 1 1] Tells the connected players to update their UI
  (if (Utilities|Name|Equal(Name) NewState "InProgress")
    (for _array_element (Variables|Default|GetConnectedControllers)
      (bind _assneaky_player_controller (Utilities|Casting|CastToSneakyPlayerController _array_element))
      (Default|SetClass _assneaky_player_controller (Variables|/Game/Blueprints/Game/SneakyPlayerController.SneakyPlayerController_C|GetClass _assneaky_player_controller))
      (Default|ConfigureUI _assneaky_player_controller))))

(event EventOnLogout
  (params (ExitingController :type Controller%20Object%20Reference))
  ;[1 1 1] Removes player controller on exit, and destroys the session with the GI instance
  (bind _asplayer_controller (Utilities|Casting|CastToPlayerController ExitingController))
  (Utilities|Array|RemoveItem (Variables|Default|GetConnectedControllers) _asplayer_controller)
  (bind _assneaky_snek_game_instance (Utilities|Casting|CastToSneakySnekGameInstance (Game|GetGameInstance)))
  (Default|DestroySession _assneaky_snek_game_instance _asplayer_controller))

(fn ConstructionScript)

(fn GetDefaultPawnClassforController
  (params (InController :type Controller%20Object%20Reference))
  (bind _assneaky_player_controller (Utilities|Casting|CastToSneakyPlayerController InController)
    (:then
      (if (Utilities|IsValidClass (.Class (Utilities|Struct|BreakDudeClass (Variables|/Game/Blueprints/Game/SneakyPlayerController.SneakyPlayerController_C|GetClass _assneaky_player_controller))))
        (return (.Class (Utilities|Struct|BreakDudeClass (Variables|/Game/Blueprints/Game/SneakyPlayerController.SneakyPlayerController_C|GetClass _assneaky_player_controller))))
        (else
          _)))
    (:CastFailed
      (Development|PrintString "Cast failed")))
  (Development|PrintString "Bad Class")
  (return "/Game/PlayerDude/Blueprints/PlayerDudeCharacter.PlayerDudeCharacter_C"))

(fn ReadytoStartMatch
  (bind _connectedcontrollers (Variables|Default|GetConnectedControllers))
  (bind _gamesettings (Variables|Default|GetGameSettings))
  (bind _numberofplayers (Utilities|Struct|BreakGameSettings _gamesettings))
  (bind _returnvalue (Utilities|Array|Length _connectedcontrollers))
  (bind _returnvalue_2 (== _numberofplayers _returnvalue))
  (bind _returnvalue_3 (Utilities|Text|ToText(Integer) _returnvalue))
  (if _returnvalue_2
    (Development|PrintText (Utilities|Text|FormatText "Starting with {players} players" _returnvalue_3))
    (CallFunction|LoadPlayers)
    (else
      (Development|PrintText (Utilities|Text|FormatText "Waiting on players {min}/{max}" _returnvalue_3 (Utilities|Text|ToText(Integer) _numberofplayers)))))
  (return _returnvalue_2))

(fn FindPlayerStart
  (params (Player :type Controller%20Object%20Reference) (IncomingName :type String))
  (bind _assneaky_player_controller (Utilities|Casting|CastToSneakyPlayerController Player)
    (:then
      (bind _outactors (Actor|GetAllActorsOfClass "/Script/Engine.PlayerStart"))
      (bind _array_element (Utilities|Array|ForEachLoopwithBreak _outactors)
        (:LoopBody
          (if (Utilities|Enum|Equal(Enum) (Utilities|String|EnumtoString (.Name (Utilities|Struct|BreakDudeClass (Variables|/Game/Blueprints/Game/SneakyPlayerController.SneakyPlayerController_C|GetClass _assneaky_player_controller)))) (Utilities|String|ToString(Name) (Variables|/Script/Engine.PlayerStart|GetPlayerStartTag _array_element)))
            (Development|PrintText (Utilities|Text|ToText(String) (Utilities|String|EnumtoString (.Name (Utilities|Struct|BreakDudeClass (Variables|/Game/Blueprints/Game/SneakyPlayerController.SneakyPlayerController_C|GetClass _assneaky_player_controller))))))
            (return _array_element)))
        (:Completed
          (bind _outactors_2 (Actor|GetAllActorsOfClass "/Script/Engine.PlayerStart" :!label _label))
          (Development|PrintText (Utilities|Text|FormatText "Bad Start {class}" (Utilities|Text|ToText(String) (Utilities|String|EnumtoString (.Name (Utilities|Struct|BreakDudeClass (Variables|/Game/Blueprints/Game/SneakyPlayerController.SneakyPlayerController_C|GetClass _assneaky_player_controller)))))))
          (return (Utilities|Array|Get(acopy) _outactors_2)))))
    (:CastFailed
      (goto _label))))

(fn SpawnDefaultPawnfor
  (params (NewPlayer :type Controller%20Object%20Reference) (StartSpot :type Actor%20Object%20Reference))
  (bind _assneaky_player_controller (Utilities|Casting|CastToSneakyPlayerController NewPlayer)
    (:then
      (if (Utilities|IsValidClass (.Class (Utilities|Struct|BreakDudeClass (Variables|/Game/Blueprints/Game/SneakyPlayerController.SneakyPlayerController_C|GetClass _assneaky_player_controller))))
        (bind _returnvalue (Game|SpawnActorfromClass (.Class (Utilities|Struct|BreakDudeClass (Variables|/Game/Blueprints/Game/SneakyPlayerController.SneakyPlayerController_C|GetClass _assneaky_player_controller))) (Transformation|GetActorTransform StartSpot) "Undefined" 0 0))
        (Default|SetClass _returnvalue (Variables|/Game/Blueprints/Game/SneakyPlayerController.SneakyPlayerController_C|GetClass _assneaky_player_controller))
        (Default|ConfigureUI _assneaky_player_controller)
        (else
          (Development|PrintString "Bad Class" :!label _label))))
    (:CastFailed
      (Development|PrintString "Cast failed")
      (goto _label)))
  (return _returnvalue))