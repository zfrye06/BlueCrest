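; Player controller that holds the player's chosen class and manages their in-game overlay UI.
; SetClass stores the class and forwards it to the controlled PlayerDudeCharacter, while SetClassServer only stores it.
; UpdateUI creates the overlay if missing, switches to game-only input and refreshes it.
; Tick repeatedly reapplies the class and refreshes the UI, and construction copies PlayerStatus from SneakySnekGameInstance.
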(event Custom|SetClass
  (params (Class :type Dude%20Class%20Structure))
  ;[1 1 1] Updates the controller class reference and sets the class on the pawn
  (Variables|Default|SetClass Class)
  (bind _asplayer_dude_character (Utilities|Casting|CastToPlayerDudeCharacter (Pawn|GetControlledPawn)))
  (Default|SetClass _asplayer_dude_character (Variables|Default|GetClass)))

(event Custom|UpdateUI
  ;[1 1 1] Configures the player's UI
  (Utilities|IsValid (Variables|Default|GetInGameOverlay)
    (:Is%20Valid
      _)
    (:Is%20Not%20Valid
      (Viewport|RemoveAllWidgets)
      (bind _returnvalue (UserInterface|CreateWidget "/Game/UI/In-Game-Overlay.In-Game-Overlay_C" self))
      (Variables|Default|SetInGameOverlay _returnvalue)
      (Input|SetInputModeGameOnly self)
      (Variables|Default|SetbShowMouseCursor false)))
  (if (UserInterface|Viewport|IsinViewport (Variables|Default|GetInGameOverlay))
    _
    (else
      (UserInterface|Viewport|AddtoPlayerScreen (Variables|Default|GetInGameOverlay))))
  (Default|UpdateUI (Variables|Default|GetInGameOverlay) self))

(event Custom|SetClassServer
  (params (Class :type Dude%20Class%20Structure))
  ;[1 1 1] Sets the class server side
  (Variables|Default|SetClass Class))

(event EventTick
  (params (DeltaSeconds :type Float%20%28single-precision%29))
  ;[1 1 1] Updates the UI every 5 seconds, not optimal, but hopefully works
  (bind _asplayer_dude_character (Utilities|Casting|CastToPlayerDudeCharacter (Pawn|GetControlledPawn)))
  (Default|SetClass _asplayer_dude_character (Variables|Default|GetClass))
  (CallFunction|UpdateUI))

(fn ConstructionScript
  (bind _assneaky_snek_game_instance (Utilities|Casting|CastToSneakySnekGameInstance (Game|GetGameInstance)))
  (Variables|Default|SetPlayerStatus (Variables|/Game/Blueprints/Game/SneakySnekGameInstance.SneakySnekGameInstance_C|GetPlayerStatus _assneaky_snek_game_instance)))