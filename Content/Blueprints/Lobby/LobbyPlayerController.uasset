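; Lobby player controller that loads a player's saved preferences and manages their lobby menu.
; Once PlayerState is valid, retried on Tick, it builds Status from a SnekPreferences save slot keyed by player name, creating one if missing.
; CallUpdate then asks LobbyGamemode to update everyone.
; Other events create the UI-only menu and refresh its player list, player count and settings, printing each player's faction and readiness for debugging.
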(event Custom|Update%20Players
  (params (Status :type Array%20of%20Player%20Status%20Structures))
  (bind _lobbymenuref (Variables|Default|GetLobbyMenuRef))
  ;[1 1 1] Attempts to update the player UI
  (Utilities|IsValid (Variables|Default|GetLobbyMenuRef)
    (:Is%20Valid
      (Default|ClearPlayersPanel _lobbymenuref)
      (Default|UpdatePlayersPanel _lobbymenuref Status)
      (for _array_element Status
        (switch Utilities|FlowControl|Switch|SwitchonFactions (.FactionPreference (Utilities|Struct|BreakPlayerStatus _array_element))
          (:NewEnumerator0
            (Variables|Default|SetFaction "Town"))
          (:NewEnumerator1
            (Variables|Default|SetFaction "Killer")))
        (Development|PrintString (Utilities|String|ToString(Text) (Utilities|Text|FormatText "{nickname}. {faction} is ready? {ready}" (.Nickname (Utilities|Struct|BreakPlayerStatus _array_element)) (Variables|Default|GetFaction) (Utilities|Text|ToText(Boolean) (.ReadyState (Utilities|Struct|BreakPlayerStatus _array_element))))))))))

(event Custom|CallUpdate
  (params (Status :type Player%20Status%20Structure))
  ;[1 1 1] Tells everyone to update
  (Variables|Default|SetStatus Status)
  (bind _aslobby_gamemode (Utilities|Casting|CastToLobbyGamemode (Game|GetGameMode)))
  (Default|EveryoneUpdate _aslobby_gamemode))

(event Custom|SetupLobbyMenu
  ;[1 1 1] Setups up the lobby menu
  (Variables|Default|SetbShowMouseCursor true)
  (bind _returnvalue (UserInterface|CreateWidget "/Game/UI/LobbyMenu.LobbyMenu_C"))
  (bind _output_get (Variables|Default|SetLobbyMenuRef _returnvalue))
  (UserInterface|Viewport|AddtoPlayerScreen _output_get)
  (Input|SetInputModeUIOnly self _output_get false))

(event Custom|UpdateSettings
  (params (Settings :type Game%20Settings%20Structure))
  ;[1 1 1] Updates the lobby menu with new settings
  (Default|UpdateSettings (Variables|Default|GetLobbyMenuRef) Settings))

(event Custom|LoadSaveGame
  (bind _playerstate (Variables|GetPlayerState))
  (bind _playername (Variables|/Script/Engine.PlayerState|GetPlayerName _playerstate))
  ;[1 1 1] Loads user preferences from the save game - Populates status defaults
  (bind _returnvalue (SaveGame|DoesSaveGameExist _playername))
  (if _returnvalue
    _
    (else
      (CallFunction|CreateSaveGame)))
  (bind _returnvalue_2 (SaveGame|LoadGamefromSlot _playername))
  (bind _assnek_preferences (Utilities|Casting|CastToSnekPreferences _returnvalue_2))
  (Variables|Default|SetStatus (Utilities|Struct|MakePlayerStatus (Variables|/Game/Blueprints/Game/SnekPreferences.SnekPreferences_C|GetPreferedFaction _assnek_preferences) false (Variables|/Game/Blueprints/Game/SnekPreferences.SnekPreferences_C|GetDefaultNickname _assnek_preferences) (Utilities|Text|ToText(String) (Variables|/Script/Engine.PlayerState|GetPlayerName (Variables|GetPlayerState))) (Ability|HasAuthority))))

(event Custom|CreateSaveGame
  (bind _playerstate (Variables|GetPlayerState))
  (bind _playername (Variables|/Script/Engine.PlayerState|GetPlayerName _playerstate))
  ;[1 1 1] Creates a save game for the given player
  (bind _returnvalue (SaveGame|CreateSaveGameObject "/Game/Blueprints/Game/SnekPreferences.SnekPreferences_C"))
  (bind _assnek_preferences (Utilities|Casting|CastToSnekPreferences _returnvalue))
  (Variables|/Game/Blueprints/Game/SnekPreferences.SnekPreferences_C|SetDefaultNickname _assnek_preferences (Utilities|Text|ToText(String) _playername))
  (SaveGame|SaveGametoSlot _assnek_preferences _playername))

(event Custom|UpdateNumberOfPlayers
  (params (CurrentPlayers :type Integer) (MaxPlayers :type Integer))
  (bind _lobbymenuref (Variables|Default|GetLobbyMenuRef))
  ;[1 1 1] Updates the number of players on the menu
  (Utilities|IsValid _lobbymenuref
    (:Is%20Valid
      (Variables|/Game/UI/LobbyMenu.LobbyMenu_C|SetPlayerCountText _lobbymenuref (Utilities|Text|FormatText "{CurPlayers}/{MaxPlayers} Players" (Utilities|Text|ToText(Integer) CurrentPlayers) (Utilities|Text|ToText(Integer) MaxPlayers))))))

(event EventBeginPlay
  ;[1 1 1] Load our player status from the game instance and add the lobby UI to the Viewport
  (Utilities|IsValid (Variables|GetPlayerState)
    (:Is%20Valid
      (CallFunction|LoadSaveGame)
      (CallFunction|CallUpdate (Variables|Default|GetStatus))
      (Variables|Default|SetHasLoaded true))))

(event EventTick
  (params (DeltaSeconds :type Float%20%28single-precision%29))
  ;[1 1 1] Keep checking if our state has loaded
  (if (not (Variables|Default|GetHasLoaded))
    (Utilities|IsValid (Variables|GetPlayerState)
      (:Is%20Valid
        (CallFunction|LoadSaveGame)
        (CallFunction|CallUpdate (Variables|Default|GetStatus))
        (Variables|Default|SetHasLoaded true)))))

(fn ConstructionScript)