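; Lobby game mode for Sneaky Snek that tracks connected players, syncs their lobby menus and starts the match.
; PostLogin registers each controller, then EveryoneUpdate pushes player count, statuses and settings to every LobbyPlayerController; logout only removes the controller.
; Settings changes are saved to the game instance and rebroadcast.
; StartGame stores the final settings, calls the loading-screen event marked multicast, and server-travels to Bluecrest.
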(event Custom|StartGame
  ;[1 1 1] Changes the map to Bluecrest
  (bind _assneaky_snek_game_instance (Utilities|Casting|CastToSneakySnekGameInstance (Game|GetGameInstance)))
  (bind _structout (Utilities|Struct|SetmembersinGameSettings (Variables|Default|GetSettings) (Variables|Default|GetCurrentPlayers)))
  (Variables|/Game/Blueprints/Game/SneakySnekGameInstance.SneakySnekGameInstance_C|SetGameSettings _assneaky_snek_game_instance _structout)
  (CallFunction|ShowLoadingtoAll)
  (Development|ExecuteConsoleCommand "servertravel /Game/Maps/bluecrest" (Game|GetPlayerController 0)))

(event Custom|EveryoneUpdate
  ;[1 1 1] Update each player controller's menu
  (bind _output_get (Variables|Default|SetCurrentPlayers (Utilities|Array|Length (Variables|Default|GetConnectedPlayers))))
  (if (> _output_get 0)
    (Utilities|Array|Clear (Variables|Default|GetPlayerStatus))
    (for _array_element (Variables|Default|GetConnectedPlayers)
      (bind _aslobby_player_controller (Utilities|Casting|CastToLobbyPlayerController _array_element))
      (Utilities|Array|Add (Variables|Default|GetPlayerStatus) (Variables|/Game/Blueprints/Lobby/LobbyPlayerController.LobbyPlayerController_C|GetStatus _aslobby_player_controller))
      (Default|UpdateNumberOfPlayers _aslobby_player_controller (Variables|Default|GetCurrentPlayers) 10)
      (Utilities|Struct|SetmembersinGameSettings (Variables|Default|GetSettings) (Variables|Default|GetCurrentPlayers)))
    (for _array_element_2 (Variables|Default|GetConnectedPlayers)
      (bind _aslobby_player_controller_2 (Utilities|Casting|CastToLobbyPlayerController _array_element_2))
      (Default|UpdatePlayers _aslobby_player_controller_2 (Variables|Default|GetPlayerStatus))
      (Default|UpdateSettings _aslobby_player_controller_2 (Variables|Default|GetSettings)))))

(event Custom|UpdateGameSettings
  (params (Settings :type Game%20Settings%20Structure))
  ;[1 1 1] Sets the new settings and instructs all the clients to update
  (bind _output_get (Variables|Default|SetSettings Settings))
  (Variables|/Game/Blueprints/Game/SneakySnekGameInstance.SneakySnekGameInstance_C|SetGameSettings (.AsSneaky%20Snek%20Game%20Instance (Utilities|Casting|CastToSneakySnekGameInstance (Game|GetGameInstance))) _output_get)
  (CallFunction|EveryoneUpdate))

(event Custom|ShowLoadingToAll
  ;[1 1 1] Multicast - Shows the loading screen on all clients screens
  (Viewport|RemoveAllWidgets)
  (bind _assneaky_snek_game_instance (Utilities|Casting|CastToSneakySnekGameInstance (Game|GetGameInstance)))
  (Default|ShowLoadingScreen _assneaky_snek_game_instance))

(event EventBeginPlay)

(event EventTick
  (params (DeltaSeconds :type Float%20%28single-precision%29)))

(event EventPostLogin
  (params (NewPlayer :type Player%20Controller%20Object%20Reference))
  ;[1 1 1] On post login add our player controller to the array and instruct others to update
  (Networking|SwitchHasAuthority
    (:Authority
      (Utilities|Array|Add (Variables|Default|GetConnectedPlayers) NewPlayer)
      (bind _aslobby_player_controller (Utilities|Casting|CastToLobbyPlayerController NewPlayer))
      (Default|SetupLobbyMenu _aslobby_player_controller)
      (CallFunction|EveryoneUpdate))))

(event EventOnLogout
  (params (ExitingController :type Controller%20Object%20Reference))
  ;[1 1 1] Remove the leaving player from the connected players array
  (bind _asplayer_controller (Utilities|Casting|CastToPlayerController ExitingController))
  (Utilities|Array|RemoveItem (Variables|Default|GetConnectedPlayers) _asplayer_controller))

(fn ConstructionScript)