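; Garage door actor that toggles between closed and open each time TriggerOpen is called, ignoring calls while it is moving.
; BeginPlay caches the mesh's world transform as closed and the OpenState component's as open.
; Tick lerps location and rotation between them using game time elapsed since the trigger over DoorOpenCloseTime.
; Movement stops once that clamped alpha reaches one, before applying that final step.
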(event Custom|TriggerOpen
  ;[1 1 1] Toggles the door state and sets the world time seconds
  ;;[1 1 1] Do nothing if moving
  (if (not (Variables|DoorStates|GetHasChangeHappened))
    (Variables|DoorStates|SetHasChangeHappened true)
    (Variables|DoorStates|SetIsOpen (not (Variables|DoorStates|GetIsOpen)))
    (Variables|DoorStates|SetWorldTimeSecondsLastPress (Utilities|Time|GetGameTimeinSeconds))))

(event EventBeginPlay
  (bind _openstate (Variables|Default|GetOpenState))
  (bind _staticmeshcomponent (Variables|Debug|GetStaticMeshComponent))
  (bind _output_get (Variables|InitialPosition|SetInitialLocation (Transformation|GetWorldLocation _staticmeshcomponent)))
  (bind _output_get_2 (Variables|InitialPosition|SetInitialRotation (Transformation|GetWorldRotation _staticmeshcomponent)))
  (Variables|OpenPosition|SetOpenRotation (Transformation|GetWorldRotation _openstate))
  (Variables|OpenPosition|SetOpenLocation (Transformation|GetWorldLocation _openstate)))

(event Collision|EventActorBeginOverlap
  (params (OtherActor :type Actor%20Object%20Reference)))

(event EventTick
  (params (DeltaSeconds :type Float%20%28single-precision%29))
  (bind _returnvalue (Utilities|Time|GetGameTimeinSeconds))
  (bind _returnvalue_2 (Utilities|Time|GetGameTimeinSeconds))
  (bind _worldtimesecondslastpress (Variables|DoorStates|GetWorldTimeSecondsLastPress))
  (bind _dooropenclosetime (Variables|Customization|GetDoorOpenCloseTime))
  (bind _staticmeshcomponent (Variables|Debug|GetStaticMeshComponent))
  (bind _staticmeshcomponent_2 (Variables|Debug|GetStaticMeshComponent))
  (bind _worldtimesecondslastpress_2 (Variables|DoorStates|GetWorldTimeSecondsLastPress))
  (bind _dooropenclosetime_2 (Variables|Customization|GetDoorOpenCloseTime))
  (bind _returnvalue_3 (- _returnvalue _worldtimesecondslastpress_2))
  (bind _returnvalue_4 (- _returnvalue_2 _worldtimesecondslastpress))
  (bind _returnvalue_5 (/ _returnvalue_3 _dooropenclosetime_2))
  (bind _returnvalue_6 (/ _returnvalue_4 _dooropenclosetime))
  (bind _returnvalue_7 (Math|Float|Clamp(Float) _returnvalue_5))
  (bind _returnvalue_8 (Math|Float|Clamp(Float) _returnvalue_6))
  (if (Variables|DoorStates|GetHasChangeHappened)
    ;[1 1 1] Calculates whether the door is still moving or not
    (Math|Float|CompareFloat (Math|Float|Clamp(Float) (/ (- (Utilities|Time|GetGameTimeinSeconds) (Variables|DoorStates|GetWorldTimeSecondsLastPress)) (Variables|Customization|GetDoorOpenCloseTime))) 1.0
      (:>
        (bind _output_get (Variables|DoorStates|SetHasChangeHappened false :!label _label)))
      (:==
        (goto _label))
      (:<
        _))
    (if _output_get
      ;[1 1 1] Chooses between closing and opening animation
      (if (Variables|DoorStates|GetIsOpen)
        ;[1 1 1] Opening door world location calculations
        (Transformation|SetWorldLocation _staticmeshcomponent (Math|Vector|Lerp(Vector) (Variables|InitialPosition|GetInitialLocation) (Variables|OpenPosition|GetOpenLocation) _returnvalue_7) false false)
        (Transformation|SetWorldRotation _staticmeshcomponent (Math|Rotator|Lerp(Rotator) (Variables|InitialPosition|GetInitialRotation) (Variables|OpenPosition|GetOpenRotation) _returnvalue_7) false false)
        (else
          ;[1 1 1] Closing door world location calculations
          (Transformation|SetWorldLocation _staticmeshcomponent_2 (Math|Vector|Lerp(Vector) (Variables|OpenPosition|GetOpenLocation) (Variables|InitialPosition|GetInitialLocation) _returnvalue_8) false false)
          (Transformation|SetWorldRotation _staticmeshcomponent_2 (Math|Rotator|Lerp(Rotator) (Variables|OpenPosition|GetOpenRotation) (Variables|InitialPosition|GetInitialRotation) _returnvalue_8) false false))))))

(fn ConstructionScript)