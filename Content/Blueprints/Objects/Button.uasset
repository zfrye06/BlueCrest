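; Button actor that a player can press with the UseItem input while standing inside its capsule.
; Entering the capsule enables input, makes the player's controller the actor's owner and shows a text render; leaving disables input and hides the text.
; Pressing UseItem routes through CallAsAuthority to fire the Pressed call, then destroys the button's owner, which the overlap sets to that controller.
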(event OnComponentBeginOverlap(Capsule)
  (params (OverlappedComponent :type Primitive%20Component%20Object%20Reference) (OtherActor :type Actor%20Object%20Reference) (OtherComp :type Primitive%20Component%20Object%20Reference) (OtherBodyIndex :type Integer) (bFromSweep :type Boolean) (SweepResult :type Hit%20Result%20Structure%20%28by%20ref%29))
  ;[1 1 1] Listen for input
  (bind _asplayer_controller (Utilities|Casting|CastToPlayerController (Game|GetInstigatorController OtherActor)))
  (Input|EnableInput _asplayer_controller)
  (Actor|SetOwner _asplayer_controller)
  (Rendering|SetVisibility (Variables|Default|GetTextRender) true false))

(event OnComponentEndOverlap(Capsule)
  (params (OverlappedComponent :type Primitive%20Component%20Object%20Reference) (OtherActor :type Actor%20Object%20Reference) (OtherComp :type Primitive%20Component%20Object%20Reference) (OtherBodyIndex :type Integer))
  ;[1 1 1] Stop listening to input once they leave
  (bind _asplayer_controller (Utilities|Casting|CastToPlayerController (Game|GetInstigatorController OtherActor)))
  (Input|DisableInput _asplayer_controller 0)
  (Rendering|SetVisibility (Variables|Default|GetTextRender) false false))

(event Custom|CallAsAuthority
  (Default|CallPressed))

(event EventBeginPlay)

(event Collision|EventActorBeginOverlap
  (params (OtherActor :type Actor%20Object%20Reference)))

(event EventTick
  (params (DeltaSeconds :type Float%20%28single-precision%29)))

(event Input|ActionEvents|InputActionUseItem
  (params (Key :type Key%20Structure :default "AnyKey"))
  (:Pressed
    (CallFunction|CallasAuthority)
    (Actor|DestroyActor (Components|GetOwner))))

(fn ConstructionScript)